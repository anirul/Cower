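; CowPawn is a pawn that glides toward the point stored in the CowController's ClickLocation and hides when damaged.
; Each Tick eases from the controlled pawn's location toward that point with a frame-time-scaled lerp, keeping its height and sweeping for collisions.
; Yaw is set instantly to face the target using Atan2 of the direction.
; Any damage hides only the static mesh, without destroying the actor or stopping movement.
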(event EventBeginPlay)

(event EventActorBeginOverlap
  (params (OtherActor :type Actor%20Object%20Reference)))

(event EventTick
  (params (DeltaSeconds :type Float%20%28single-precision%29))
  (bind _returnvalue (Game|GetPlayerController 0))
  (bind _returnvalue_2 (Pawn|GetControlledPawn _returnvalue))
  (bind _returnvalue_3 (Transformation|GetActorLocation _returnvalue_2))
  (bind _ascow_controller (Utilities|Casting|CastToCowController _returnvalue))
  (Transformation|SetActorLocationAndRotation (Math|Vector|Lerp(Vector) _returnvalue_3 (Math|Vector|MakeVector (.X (Math|Vector|BreakVector (Variables|/Game/BluePrints/CowController.CowController_C|GetClickLocation _ascow_controller))) (.Y (Math|Vector|BreakVector (Variables|/Game/BluePrints/CowController.CowController_C|GetClickLocation _ascow_controller))) (.Z (Math|Vector|BreakVector _returnvalue_3))) (* DeltaSeconds 2.0)) (Math|Rotator|MakeRotator 0.0 0.0 (Class|KismetMathLibrary|DegAtan2 (.Y (Math|Vector|BreakVector (Math|Vector|Normalize (- (Variables|/Game/BluePrints/CowController.CowController_C|GetClickLocation _ascow_controller) _returnvalue_3)))) (.X (Math|Vector|BreakVector (Math|Vector|Normalize (- (Variables|/Game/BluePrints/CowController.CowController_C|GetClickLocation _ascow_controller) _returnvalue_3)))))) true))

(event Game|Damage|EventAnyDamage
  (params (Damage :type Float%20%28single-precision%29) (DamageType :type Damage%20Type%20Object%20Reference) (InstigatedBy :type Controller%20Object%20Reference) (DamageCauser :type Actor%20Object%20Reference))
  (Rendering|SetVisibility (Variables|Default|GetStaticMesh) false false))

(fn ConstructionScript)