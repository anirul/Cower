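; CowController is a click-to-move player controller that sends its controlled pawn to a point picked under the cursor or finger.
; Each Tick runs gated cursor and finger traces on the Visibility channel; first-finger press and release toggle touch tracking, while no key event drives the cursor gate.
; MoveToHitLocation ignores hits closer to the pawn than MinClickDistance, otherwise calls SimpleMoveToLocation and stores ClickLocation.
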(event `self.ReceiveBeginPlay`)

(event `self.ReceiveTick`
  (params (DeltaSeconds :type "Float (single-precision)"))
  ;[1 1 1] Click and go there
  (`|ExecutionSequence`
    (:`then_0`
      (`/Engine/EditorBlueprintResources/StandardMacros.Gate` true ; While key is pressed...
        (:`Exit`
          (`self.MoveToHitLocation` (`self.GetHitResultUnderCursorByChannel` "TraceTypeQuery1")))))
    (:`then_1`
      (`/Engine/EditorBlueprintResources/StandardMacros.Gate` true :!label _label ; While finger is touching...
        (:`Exit`
          (`self.MoveToHitLocation` (`self.GetHitResultUnderFingerByChannel` (stale `InputTouch` FingerIndex) "TraceTypeQuery1")))))))

(event `InputTouch`
  (params (Location :type "Vector Structure") (FingerIndex :type "ETouchIndex Enum" :default "Touch1"))
  (bind _returnvalue (`|EnumEquality` FingerIndex "Touch1"))
  ;[1 1 1] Click and go there
  (:`Pressed`
    (if _returnvalue
      (goto _label :!via `Open`)))
  (:`Released`
    (if _returnvalue
      (goto _label :!via `Close`))))

(fn `MoveToHitLocation`
  (params (Hit :type "HitResult Structure"))
  (bind (_bblockinghit _binitialoverlap _time _location) (`GameplayStatics.BreakHitResult` Hit))
  (if (>= (`KismetMathLibrary.VSize` (- (`self.K2_GetActorLocation` (`self.K2_GetPawn`)) _location)) (`self.MinClickDistance`))
    (`NavigationSystem.SimpleMoveToLocation` self _location) ; Send the destination point to the character
    (set `self.ClickLocation` _location)))

(fn `UserConstructionScript`)