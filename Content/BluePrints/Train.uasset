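; Train is a moving hazard actor that travels in a straight line and harms the player when it hits a CowPawn.
; Tick moves it along Direction at Speed with a swept location update, and BeginPlay destroys it after a fixed delay.
; When its StaticMesh begins overlapping a CowPawn, it applies damage to player pawn 0 and prints a Game Over message.
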(event `self.ReceiveBeginPlay`
  (`KismetSystemLibrary.Delay` 10.0)
  (`self.K2_DestroyActor`))

(event `self.ReceiveActorBeginOverlap`
  (params (OtherActor :type "Actor Object Reference")))

(event `self.ReceiveTick`
  (params (DeltaSeconds :type "Float (single-precision)"))
  (`self.K2_SetActorLocation` (+ (`self.K2_GetActorLocation`) (* (* (`self.Direction`) DeltaSeconds) (`self.Speed`))) true))

(event `self.StaticMesh.OnComponentBeginOverlap`
  (params (OtherActor :type "Actor Object Reference") (OtherComp :type "PrimitiveComponent Object Reference") (OtherBodyIndex :type Integer) (bFromSweep :type Boolean) (SweepResult :type "HitResult Structure (by ref)"))
  (cast `/Game/BluePrints/CowPawn` OtherActor)
  (`GameplayStatics.ApplyDamage` (`GameplayStatics.GetPlayerPawn` 0) 10.0)
  (`KismetSystemLibrary.PrintString` "Game Over" true true (struct :`R` 1.0 :`G` 0.008069 :`A` 1.0)))

(fn `UserConstructionScript`)